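; Openable component that swings its owning actor, apparently a door, between closed and open rotations with matching sounds.
; Each Tick it reads the Open flag and snaps the owner to the matching hard-coded world rotation, with no interpolation.
; Current-rotation checks make the snap and sound fire only on a state change, and only for owners sitting at one of those two rotations.
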(event EventTick
  (params (DeltaSeconds :type Float%20%28single-precision%29))
  (bind _returnvalue (Components|GetOwner))
  (bind _returnvalue_2 (Components|GetOwner))
  (bind _returnvalue_3 (Transformation|GetActorLocation _returnvalue_2))
  (if (Variables|Default|GetOpen)
    (if (Utilities|Operators|EqualEqual (Transformation|GetActorRotation _returnvalue_2) "0,0.000000,0" 0.0) ; Only rotate and play noise if necessary
      (Transformation|SetActorRotation _returnvalue_2 "0,10.000000, 0")
      (Audio|PlaySoundatLocation "/Game/Audio/Door_Open_2.Door_Open_2" _returnvalue_3 "0, 0, 0" 1.0 1.0 0.0 0 0 0 0))
    (elif (Utilities|Operators|EqualEqual (Transformation|GetActorRotation _returnvalue) "0,10.000000,0" 1.0) ; Only rotate and play noise if necessary
      (Transformation|SetActorRotation _returnvalue "0,0.000000, 0")
      (Audio|PlaySoundatLocation "/Game/Audio/Door_Close_2.Door_Close_2" _returnvalue_3 "0, 0, 0" 1.0 1.0 0.0 0 0 0 0))))