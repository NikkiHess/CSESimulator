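; BPDialogue is a short-lived actor that shows a widget component, likely a dialogue bubble, in the world.
; Each tick it rotates the widget to face the player camera using a look-at rotation.
; On its first tick it sets a flag and starts a three-second delay, then destroys itself.
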(event EventTick
  (params (DeltaSeconds :type Float%20%28single-precision%29))
  (Transformation|SetWorldRotation (Variables|Default|GetWidget) (Math|Rotator|FindLookatRotation (Transformation|GetWorldLocation (Variables|Default|GetWidget)) (Camera|GetCameraLocation (Game|GetPlayerCameraManager 0))) false false)
  (if (not (Variables|Default|GetExists))
    (Variables|Default|SetExists true)
    (Utilities|FlowControl|Delay 3.0)
    (Actor|DestroyActor)))

(fn ConstructionScript)