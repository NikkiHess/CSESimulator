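; BPLightFlicker is a component-style Blueprint that makes its owning actor randomly blink out, imitating a flickering light.
; Each Tick, a visible, non-flickering owner has a roughly one percent chance to be hidden with a quiet, high-pitched switch sound.
; After a one-second delay the actor reappears, with a flag blocking overlapping flickers.
; The random roll runs per frame, so flicker frequency depends on frame rate.
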(event EventTick
  (params (DeltaSeconds :type Float%20%28single-precision%29))
  (bind _returnvalue (Components|GetOwner))
  (if (Math|Boolean|ANDBoolean (not (Variables|Default|GetIs%20Flickering)) (> (Math|Random|RandomFloat) 0.99) (not (Variables|/Script/Engine.Actor|GetbHidden (Components|GetOwner))))
    (Rendering|SetActorHiddenInGame _returnvalue true)
    (Audio|PlaySoundatLocation "/Game/Audio/Light_Switch.Light_Switch" (Transformation|GetActorLocation _returnvalue) "0, 0, 0" 0.25 2.0 0.0 0 0 0 0)
    (Variables|Default|SetIs%20Flickering true)
    (Utilities|FlowControl|Delay 1.0)
    (Rendering|SetActorHiddenInGame _returnvalue false)
    (Variables|Default|SetIs%20Flickering false)))